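; Meeple is an AI-moved pawn that travels to a random zone when play begins.
; On BeginPlay it caches the DFS_GameState and the level's NavMeshBoundsVolume, then asks the game state for a random zone and stores it as its target.
; An AI MoveTo sends it to that zone and prints a debug message on success or failure.
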(event `self.ReceiveBeginPlay`
  (bind _asdfs_game_state (cast `/Game/Blueprints/Base/DFS_GameState` (`GameplayStatics.GetGameState`)))
  (bind _output_get (set `self.GameStateRef` _asdfs_game_state))
  (bind _returnvalue (`GameplayStatics.GetActorOfClass` "/Script/NavigationSystem.NavMeshBoundsVolume"))
  (set `self.NavMeshRef` _returnvalue)
  (bind _randomzone (`/Game/Blueprints/Base/DFS_GameState.GetRandomZone` _output_get))
  (bind _output_get_2 (set `self.TargetZone` _randomzone))
  (`|AIMoveTo` self (0.0 0.0 0.0) _output_get_2
    (:`OnSuccess`
      (`KismetSystemLibrary.PrintText` "SUCCEDED to get to target" true true (struct :`G` 0.203125 :`B` 0.028878 :`A` 1.0)))
    (:`OnFail`
      (`KismetSystemLibrary.PrintText` "FAILED to get to target" true true (struct :`R` 1.0 :`G` 0.145833 :`B` 0.173379 :`A` 1.0)))))

(fn `UserConstructionScript`)