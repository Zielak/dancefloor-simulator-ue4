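; Game state that indexes the level's tagged zone trigger volumes and serves random picks from them.
; On BeginPlay, InitAllZones sorts the volumes into Drinks, Food, Entrance and Dancefloor arrays, printing debug paths and counts.
; GetRandomZone picks a random category then a volume; GetRandomZoneOfType picks within a given category, falling back to GetRandomZone.
; Random indices use array length as inclusive maximum, so can overrun by one.
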(event `self.ReceiveBeginPlay`
  (`self.InitAllZones`))

(event `self.ReceiveTick`
  (params (DeltaSeconds :type "Float (single-precision)")))

(fn `GetRandomZone`
  (returns (RandomZone :type "TriggerVolume Object Reference"))
  (locals (CountZones :type Integer) (ChosenZone :type "TriggerVolume Object Reference"))
  (switch `int` (`KismetMathLibrary.RandomIntegerInRange` 0 3)
    (:`0`
      (set `local.ChosenZone` (`|GetArrayItem` (`self.ZonesDrinks`) (`KismetMathLibrary.RandomIntegerInRange` 0 (`KismetArrayLibrary.Array_Length` (`self.ZonesDrinks`))))))
    (:`1`
      (set `local.ChosenZone` (`|GetArrayItem` (`self.ZonesFood`) (`KismetMathLibrary.RandomIntegerInRange` 0 (`KismetArrayLibrary.Array_Length` (`self.ZonesFood`))))))
    (:`2`
      (set `local.ChosenZone` (`|GetArrayItem` (`self.ZonesEntrance`) (`KismetMathLibrary.RandomIntegerInRange` 0 (`KismetArrayLibrary.Array_Length` (`self.ZonesEntrance`))))))
    (:`3`
      (set `local.ChosenZone` (`|GetArrayItem` (`self.ZonesDancefloor`) (`KismetMathLibrary.RandomIntegerInRange` 0 (`KismetArrayLibrary.Array_Length` (`self.ZonesDancefloor`)))))))
  (`KismetSystemLibrary.PrintString` (`KismetStringLibrary.Concat_StrStr` "Chosen zone: " (`KismetSystemLibrary.GetDisplayName` (`local.ChosenZone`))) true true (struct :`R` 1.0 :`G` 0.338542 :`B` 0.969568 :`A` 1.0) 30.0)
  (return (`local.ChosenZone`)))

(fn `GetRandomZoneOfType`
  (params (`Zone Tag` :type Name))
  (returns (Zone :type "TriggerVolume Object Reference"))
  (locals (ReturnValue :type "TriggerVolume Object Reference"))
  (switch `name` `Zone Tag`
    (:`Default`
      (bind _randomzone (`self.GetRandomZone`))
      (set `local.ReturnValue` _randomzone))
    (:`drinks`
      (set `local.ReturnValue` (`|GetArrayItem` (`self.ZonesDrinks`) (`KismetMathLibrary.RandomIntegerInRange` 0 (`KismetArrayLibrary.Array_Length` (`self.ZonesDrinks`))))))
    (:`food`
      (set `local.ReturnValue` (`|GetArrayItem` (`self.ZonesFood`) (`KismetMathLibrary.RandomIntegerInRange` 0 (`KismetArrayLibrary.Array_Length` (`self.ZonesFood`))))))
    (:`entrance`
      (set `local.ReturnValue` (`|GetArrayItem` (`self.ZonesEntrance`) (`KismetMathLibrary.RandomIntegerInRange` 0 (`KismetArrayLibrary.Array_Length` (`self.ZonesEntrance`))))))
    (:`dancefloor`
      (set `local.ReturnValue` (`|GetArrayItem` (`self.ZonesDancefloor`) (`KismetMathLibrary.RandomIntegerInRange` 0 (`KismetArrayLibrary.Array_Length` (`self.ZonesDancefloor`)))))))
  (return (`local.ReturnValue`)))

(fn `InitAllZones`
  (locals (TriggerVolume :type "TriggerVolume Object Reference") (FoundZones :type "Array of TriggerVolume Object Reference"))
  (bind _triggervolume (`local.TriggerVolume`))
  (bind _outactors (`GameplayStatics.GetAllActorsOfClassWithTag` "/Script/Engine.TriggerVolume" "zone"))
  (bind _output_get (set `local.FoundZones` _outactors))
  (for _array_element _output_get
    (bind _output_get_2 (set `local.TriggerVolume` _array_element))
    (`KismetSystemLibrary.PrintString` (`KismetSystemLibrary.GetPathName` _output_get_2) true true (struct :`G` 0.66 :`B` 1.0 :`A` 1.0) 30.0)
    (for _array_element_2 _
      (switch `name` _array_element_2
        (:`drinks`
          (`KismetArrayLibrary.Array_Add` (`self.ZonesDrinks`) _triggervolume))
        (:`food`
          (`KismetArrayLibrary.Array_Add` (`self.ZonesFood`) _triggervolume))
        (:`entrance`
          (`KismetArrayLibrary.Array_Add` (`self.ZonesEntrance`) _triggervolume))
        (:`dancefloor`
          (`KismetArrayLibrary.Array_Add` (`self.ZonesDancefloor`) _triggervolume)))))
  (`KismetSystemLibrary.PrintText` (`KismetTextLibrary.Conv_StringToText` (`KismetStringLibrary.Concat_StrStr` (`KismetStringLibrary.Concat_StrStr` " \ndrinks:" (`KismetStringLibrary.Conv_IntToString` (`KismetArrayLibrary.Array_Length` (`self.ZonesDrinks`)))) (`KismetStringLibrary.Concat_StrStr` " \nfood:" (`KismetStringLibrary.Conv_IntToString` (`KismetArrayLibrary.Array_Length` (`self.ZonesFood`)))) (`KismetStringLibrary.Concat_StrStr` " \nentrance:" (`KismetStringLibrary.Conv_IntToString` (`KismetArrayLibrary.Array_Length` (`self.ZonesEntrance`)))) (`KismetStringLibrary.Concat_StrStr` " \ndancefloor:" (`KismetStringLibrary.Conv_IntToString` (`KismetArrayLibrary.Array_Length` (`self.ZonesDancefloor`)))))) true true (struct :`G` 0.66 :`B` 1.0 :`A` 1.0) 5.0))

(fn `UserConstructionScript`)